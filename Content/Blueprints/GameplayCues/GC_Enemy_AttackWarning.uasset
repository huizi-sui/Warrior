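; Gameplay cue that shows an unblockable-attack warning effect on an enemy when executed.
; Spawns the NS_UnbloackableWarning Niagara system 100 units ahead of the target's eye viewpoint, oriented along its forward vector.
; It then attaches the effect to the target's root with KeepRelative rules, so the world-space spawn transform is reinterpreted as relative to the root.
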(fn `OnExecute`
  (params (MyTarget :type "Actor Object Reference") (Parameters :type "GameplayCueParameters Structure (by ref)"))
  (returns (ReturnValue :type Boolean))
  (bind _returnvalue (`NiagaraFunctionLibrary.SpawnSystemAtLocation` null "/Game/Assets/Niagara/Warning/NS_UnbloackableWarning.NS_UnbloackableWarning" (+ (`Actor.GetActorEyesViewPoint` (`local.MyTarget`)) (* (`Actor.GetActorForwardVector` (`local.MyTarget`)) 100.0)) (`KismetMathLibrary.Conv_VectorToRotator` (`Actor.GetActorForwardVector` (`local.MyTarget`)))))
  (`SceneComponent.K2_AttachToComponent` _returnvalue (`Actor.RootComponent` (`local.MyTarget`)) "None" "KeepRelative" "KeepRelative" "KeepRelative" true)
  (return (`parent.OnExecute` (`local.MyTarget`) (`local.Parameters`))))